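; BP_AuraPlayerCharacter is the Aura player character Blueprint, adding motion-warped facing and overlap-driven fade handling.
; SetFacingTagetLocation writes the given location to the Motion Warping component's FacingTarget warp target.
; Two fade triggers each feed their own AuraFadeSource, pushing actors on begin overlap and popping them on end overlap.
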(event OnComponentBeginOverlap(FadeTrigger)
  (params (OverlappedComponent :type Primitive%20Component%20Object%20Reference) (OtherActor :type Actor%20Object%20Reference) (OtherComp :type Primitive%20Component%20Object%20Reference) (OtherBodyIndex :type Integer) (bFromSweep :type Boolean) (SweepResult :type Hit%20Result%20Structure%20%28by%20ref%29))
  (Class|AuraFadeSourceComponent|PushActor (Variables|Default|GetAuraFadeSource) OtherActor))

(event OnComponentEndOverlap(FadeTrigger)
  (params (OverlappedComponent :type Primitive%20Component%20Object%20Reference) (OtherActor :type Actor%20Object%20Reference) (OtherComp :type Primitive%20Component%20Object%20Reference) (OtherBodyIndex :type Integer))
  (Class|AuraFadeSourceComponent|PopActor (Variables|Default|GetAuraFadeSource) OtherActor))

(event OnComponentBeginOverlap(FadeTrigger2)
  (params (OverlappedComponent :type Primitive%20Component%20Object%20Reference) (OtherActor :type Actor%20Object%20Reference) (OtherComp :type Primitive%20Component%20Object%20Reference) (OtherBodyIndex :type Integer) (bFromSweep :type Boolean) (SweepResult :type Hit%20Result%20Structure%20%28by%20ref%29))
  (Class|AuraFadeSourceComponent|PushActor (Variables|Default|GetAuraFadeSource2) OtherActor))

(event OnComponentEndOverlap(FadeTrigger2)
  (params (OverlappedComponent :type Primitive%20Component%20Object%20Reference) (OtherActor :type Actor%20Object%20Reference) (OtherComp :type Primitive%20Component%20Object%20Reference) (OtherBodyIndex :type Integer))
  (Class|AuraFadeSourceComponent|PopActor (Variables|Default|GetAuraFadeSource2) OtherActor))

(event EventSetFacingTagetLocation
  (params (TargetLocation :type Vector%20%28by%20ref%29 :default "0, 0, 0"))
  (Class|MotionWarpingComponent|AddorUpdateWarpTargetfromLocation (Variables|Default|GetMotionWarping) "FacingTarget" TargetLocation))

(fn ConstructionScript)