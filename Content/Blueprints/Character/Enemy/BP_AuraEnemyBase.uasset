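; Base enemy character Blueprint that supplies shared visual and motion behavior for enemies.
; Tick draws a debug capsule around the collision capsule when debug info is enabled and the enemy is highlighted.
; A timeline drives the Dissolve scalar on supplied dynamic material instances for a dissolve effect.
; A facing event feeds a target location to Motion Warping as the "Facing Target" warp target.
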(event EventStartDissolveTimeline
  (params (DynamicMaterialInstances :type Array%20of%20Material%20Instance%20Dynamic%20Object%20References))
  (bind _dissolve (Timeline|DissolveTimeline PlayFromStart)
    (:Update
      (for _array_element DynamicMaterialInstances
        (Rendering|Material|SetScalarParameterValue _array_element "Dissolve" _dissolve :!class /Script/Engine.MaterialInstanceDynamic)))))

(event EventSetFacingTagetLocation
  (params (TargetLocation :type Vector%20%28by%20ref%29 :default "0, 0, 0"))
  (Class|MotionWarpingComponent|AddorUpdateWarpTargetfromLocation (Variables|Default|GetMotionWarping) "Facing Target" TargetLocation))

(event EventTick
  (params (DeltaSeconds :type Float%20%28single-precision%29))
  (bind _capsulecomponent (Variables|Default|GetCapsuleComponent))
  (if (Variables|Debug|GetShowDebugInfo)
    (if (Variables|Default|GetbHighlighted)
      (Rendering|Debug|DrawDebugCapsule (Transformation|GetWorldLocation _capsulecomponent) (Variables|/Script/Engine.CapsuleComponent|GetCapsuleHalfHeight _capsulecomponent) (Variables|/Script/Engine.CapsuleComponent|GetCapsuleRadius _capsulecomponent) "0, 0, 0" "(R=1.000000,G=0.000000,B=0.063568,A=1.000000)" 0.0 0.0))))

(fn ConstructionScript)