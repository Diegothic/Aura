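; Fire pillar actor whose light flickers like a flame.
; On BeginPlay it picks a random time offset so separate instances do not flicker in sync.
; Each Tick, 1D Perlin noise over game time drives the FireLight intensity around a base value.
; A second, slower noise sample blends the light color between two warm orange tones.
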(event EventTick
  (params (DeltaSeconds :type Float%20%28single-precision%29))
  (bind _returnvalue (Utilities|Time|GetGameTimeinSeconds))
  (bind _firelight (Variables|Default|GetFireLight))
  (bind _randoffset (Variables|Default|GetRandOffset))
  (bind _returnvalue_2 (+ _returnvalue _randoffset))
  (Rendering|Components|Light|SetIntensity _firelight (+ (* (Class|KismetMathLibrary|PerlinNoise1D (* _returnvalue_2 5.0)) 7e+01) (Variables|Default|GetBaseIntensity)))
  (Rendering|Components|Light|SetLightColor _firelight (Math|Color|Lerp(LinearColor) "(R=1.000000,G=0.174922,B=0.023153,A=1.000000)" "(R=1.000000,G=0.207484,B=0.023153,A=1.000000)" (/ (+ (Class|KismetMathLibrary|PerlinNoise1D (* _returnvalue_2 3.0)) 1.0) 2.0)) true))

(event EventBeginPlay
  (Variables|Default|SetRandOffset (* (Math|Random|RandomFloat) 1e+03)))

(fn ConstructionScript)