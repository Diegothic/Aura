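; Player controller for Aura that sets up audio listening for the possessed character and provides debug hotkeys.
; On possess, it overrides the audio listener's attenuation location to follow the character's mesh, so distance falloff is measured from the character.
; The H and J keys apply debug Gameplay Effects to the controlled pawn's Ability System Component to deplete health and mana respectively.
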(event EventPossess
  (params (PossessedPawn :type Pawn%20Object%20Reference))
  (bind _ascharacter (Utilities|Casting|CastToCharacter PossessedPawn))
  (Class|PlayerController|SetAudioListenerAttenuationOverride (Variables|/Script/Engine.Character|GetMesh _ascharacter) "0, 0, 0"))

(event Input|KeyboardEvents|H
  (params (Key :type Key%20Structure :default "None"))
  (:Pressed
    (GameplayEffects|ApplyGameplayEffectToSelf :self (Ability|GetAbilitySystemComponent (Pawn|GetControlledPawn)) :GameplayEffectClass "/Game/Blueprints/Effects/Debug/GE_DebugDepleteHealth.GE_DebugDepleteHealth_C")))

(event Input|KeyboardEvents|J
  (params (Key :type Key%20Structure :default "None"))
  (:Pressed
    (GameplayEffects|ApplyGameplayEffectToSelf :self (Ability|GetAbilitySystemComponent (Pawn|GetControlledPawn)) :GameplayEffectClass "/Game/Blueprints/Effects/Debug/GE_DebugDepleteMana.GE_DebugDepleteMana_C")))

(fn ConstructionScript)