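; GA_HitReact is a Gameplay Ability that plays a hit reaction on the avatar.
; On activation it applies the GE_HitReact effect to the owner and plays the montage supplied by the avatar's CombatInterface.
; The ability ends when the montage completes and cancels if it is interrupted, cancelled or the interface cast fails.
; OnEndAbility removes the stored effect handle if still active, so the effect lasts only as long as the ability.
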(event Ability|EventActivateAbility
  (bind _returnvalue (Ability|ApplyGameplayEffectToOwner "/Game/Blueprints/AbilitySystem/GameplayEffect/GE_HitReact.GE_HitReact_C"))
  (Variables|Default|SetHitReactEffectHandle _returnvalue)
  (bind _ascombat_interface (Utilities|Casting|CastToCombatInterface (Ability|GetAvatarActorfromActorInfo))
    (:then
      (|PlayMontageandWaitProxy "None" (Class|CombatInterface|GetHitReactMontage _ascombat_interface) 1.0 "None" true 1.0 0.0 false
        (:OnCompleted
          (Ability|EndAbility))
        (:OnInterrupted
          (Ability|CancelAbility :!label _label))
        (:OnCancelled
          (goto _label))))
    (:CastFailed
      (Ability|CancelAbility))))

(event Ability|EventOnEndAbility
  (params (bWasCancelled :type Boolean))
  (bind _returnvalue (Class|AbilitySystemBlueprintLibrary|IsActiveGameplayEffectHandleActive (Variables|Default|GetHitReactEffectHandle)))
  (if _returnvalue
    (GameplayEffects|RemoveActiveGameplayEffect (Ability|GetAbilitySystemComponentfromActorInfo) (Variables|Default|GetHitReactEffectHandle) -1)))