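; Ranged attack gameplay ability for enemies that fires a projectile at their combat target.
; On activation it caches the target's location, sets it as the facing location through the combat interface, then synchronously loads and plays a random tagged attack montage.
; The montage's gameplay event triggers the projectile, aimed slightly above the cached location, and the ability ends when the montage completes, is interrupted or is cancelled.
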(event Ability|EventActivateAbility
  (Utilities|FlowControl|Sequence
    (:then_0
      (bind _asaura_enemy_interface (Utilities|Casting|CastToAuraEnemyInterface (Ability|GetAvatarActorfromActorInfo)))
      (Utilities|IsValid (Class|AuraEnemyInterface|GetCombatTarget _asaura_enemy_interface)
        (:Is%20Valid
          (Variables|Default|SetTargetLocation (Transformation|GetActorLocation (Class|AuraEnemyInterface|GetCombatTarget _asaura_enemy_interface))))))
    (:then_1
      (bind _ascombat_interface (Utilities|Casting|CastToCombatInterface (Ability|GetAvatarActorfromActorInfo)))
      (Class|CombatInterface|SetFacingTagetLocation _ascombat_interface (Variables|Default|GetTargetLocation)))
    (:then_2
      (Variables|Default|SetAttackTaggedMontage (Class|AuraDamageGameplayAbility|GetRandomAttackMontage))
      (bind _returnvalue (Utilities|LoadAssetBlocking (.Montage (Utilities|Struct|BreakAuraTaggedMontage (Variables|Default|GetAttackTaggedMontage)))))
      (bind _asanim_montage (Utilities|Casting|CastToAnimMontage _returnvalue))
      (|PlayMontageandWaitProxy "None" _asanim_montage 1.0 "None" false 1.0 0.0 false
        (:then
          (Ability|Tasks|WaitGameplayEvent (.MontageTag (Utilities|Struct|BreakAuraTaggedMontage (Variables|Default|GetAttackTaggedMontage))) 0
            (:EventReceived
              (Class|AuraProjectileSpell|SpawnProjectile (+ (Variables|Default|GetTargetLocation) (* (Math|Vector|VectorUp) "0.000000,0.000000,100.000000"))))))
        (:OnCompleted
          (Ability|EndAbility :!label _label))
        (:OnInterrupted
          (goto _label))
        (:OnCancelled
          (goto _label))))))