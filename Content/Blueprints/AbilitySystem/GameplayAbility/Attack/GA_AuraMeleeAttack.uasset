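; Melee attack gameplay ability for Aura enemies that turns toward the combat target and plays a random attack montage.
; A gameplay event matching the montage's socket tag triggers a small radius check at that combat socket, damaging non-friendly actors and firing an impact gameplay cue.
; Finding any actor also briefly freezes the attacker through custom time dilation for hitstop.
; The ability ends when the montage completes, is interrupted or is cancelled.
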(event Custom|OnHitstopEnd
  (Variables|/Script/Engine.Actor|SetCustomTimeDilation (Ability|GetAvatarActorfromActorInfo) 1.0))

(event Ability|EventActivateAbility
  (Utilities|FlowControl|Sequence
    (:then_0
      (bind _asaura_enemy_interface (Utilities|Casting|CastToAuraEnemyInterface (Ability|GetAvatarActorfromActorInfo)))
      (Utilities|IsValid (Class|AuraEnemyInterface|GetCombatTarget _asaura_enemy_interface)
        (:Is%20Valid
          (Variables|Default|SetTarget%20Location (Transformation|GetActorLocation (Class|AuraEnemyInterface|GetCombatTarget _asaura_enemy_interface))))))
    (:then_1
      (bind _ascombat_interface (Utilities|Casting|CastToCombatInterface (Ability|GetAvatarActorfromActorInfo)))
      (Class|CombatInterface|SetFacingTagetLocation _ascombat_interface (Variables|Default|GetTarget%20Location)))
    (:then_2
      (Variables|Default|SetAttackTaggedMontage (Class|AuraDamageGameplayAbility|GetRandomAttackMontage))
      (bind _returnvalue (Utilities|LoadAssetBlocking (.Montage (Utilities|Struct|BreakAuraTaggedMontage (Variables|Default|GetAttackTaggedMontage)))))
      (bind _asanim_montage (Utilities|Casting|CastToAnimMontage _returnvalue))
      (|PlayMontageandWaitProxy "None" _asanim_montage 1.0 "None" true 1.0 0.0 false
        (:then
          (Ability|Tasks|WaitGameplayEvent (.SocketTag (Utilities|Struct|BreakAuraTaggedMontage (Variables|Default|GetAttackTaggedMontage))) 0 true
            (:EventReceived
              (bind _ascombat_interface_2 (Utilities|Casting|CastToCombatInterface (Ability|GetAvatarActorfromActorInfo)))
              (bind _output_get (Variables|Default|SetCombatSocketLocation (Class|CombatInterface|GetCombatSocketLocation _ascombat_interface_2 (.SocketTag (Utilities|Struct|BreakAuraTaggedMontage (Variables|Default|GetAttackTaggedMontage))))))
              (bind _outoverlappingactors (Class|AuraAbilitySystemStatics|GetAliveCombatActorsinRadius _output_get 45.0 (Utilities|Array|MakeArray (Ability|GetAvatarActorfromActorInfo))))
              (if (not (Utilities|Array|IsEmpty _outoverlappingactors))
                (Utilities|FlowControl|Sequence
                  (:then_1
                    (for _array_element _outoverlappingactors
                      (Utilities|IsValid _array_element
                        (:Is%20Valid
                          (if (not (Class|AuraAbilitySystemStatics|AreActorsFriendly _array_element (Ability|GetAvatarActorfromActorInfo)))
                            (Utilities|FlowControl|Sequence
                              (:then_0
                                (Class|AuraDamageGameplayAbility|CauseDamage _array_element))
                              (:then_1
                                (Class|GameplayAbility|ExecuteGameplayCuewithParams "(TagName=\"GameplayCue.MeleeHitImpact\")" (Ability|GameplayCue|MakeGameplayCueParameters :AggregatedSourceTags (GameplayTags|MakeGameplayTagContainerfromArray (Utilities|Array|MakeArray (.MontageTag (Utilities|Struct|BreakAuraTaggedMontage (Variables|Default|GetAttackTaggedMontage))) (.SocketTag (Utilities|Struct|BreakAuraTaggedMontage (Variables|Default|GetAttackTaggedMontage))))) :Location (Variables|Default|GetCombatSocketLocation) :Instigator (Ability|GetAvatarActorfromActorInfo) :SourceObject _array_element))))))))
                    (Variables|/Script/Engine.Actor|SetCustomTimeDilation (Ability|GetAvatarActorfromActorInfo) 0.0)
                    (Utilities|Time|SetTimerbyEvent (delegate Custom|OnHitstopEnd) 0.1)))))))
        (:OnCompleted
          (Ability|EndAbility :!label _label))
        (:OnInterrupted
          (goto _label))
        (:OnCancelled
          (goto _label))))))